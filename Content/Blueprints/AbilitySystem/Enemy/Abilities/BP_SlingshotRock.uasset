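; BP_SlingshotRock is a rock actor among the enemy ability assets, likely a slingshot projectile, that tumbles visually while it exists.
; BeginPlay sets yaw, pitch and roll rates through random-range calls whose identical bounds make the spin fixed.
; Tick scales these rates by delta time and applies them as local rotation to RockMesh.
; The graphs here contain no movement, collision or damage logic.
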(event EventBeginPlay
  (bind _returnvalue (Math|Random|RandomFloatinRange -5e+02 -5e+02))
  (Variables|Default|SetYawRotationRate _returnvalue)
  (Variables|Default|SetPitchRotationRate _returnvalue)
  (Variables|Default|SetRollRotationRate _returnvalue))

(event Collision|EventActorBeginOverlap
  (params (OtherActor :type Actor%20Object%20Reference)))

(event EventTick
  (params (DeltaSeconds :type Float%20%28single-precision%29))
  (Transformation|AddLocalRotation (Variables|Default|GetRockMesh) (Math|Rotator|MakeRotator (* DeltaSeconds (Variables|Default|GetRollRotationRate)) (* DeltaSeconds (Variables|Default|GetPitchRotationRate)) (* DeltaSeconds (Variables|Default|GetYawRotationRate))) false false))

(fn ConstructionScript)