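; BP_FlamePillar is a flame pillar actor whose FireLight flickers continuously with varied intensity.
; From BeginPlay it randomly plays one of two intensity timelines, then picks again whenever one finishes, forming an endless non-fixed loop.
; Each timeline update feeds ScaleFlameIntensity, which multiplies the curve value by BaseIntensity and applies it to the light.
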(event Custom|StartTimeLine1
  (bind _flameintensity (Timeline|FlameIntensityTimeline1 PlayFromStart)
    (:Update
      (CallFunction|ScaleFlameIntensity _flameintensity))
    (:Finished
      (CallFunction|ChooseTimeline))))

(event Custom|StartTimeLine2
  (bind _flameintensity (Timeline|FlameIntensityTimeline2 PlayFromStart)
    (:Update
      (CallFunction|ScaleFlameIntensity _flameintensity))
    (:Finished
      (CallFunction|ChooseTimeline))))

(event Custom|ChooseTimeline
  (switch int (Math|Random|RandomIntegerinRange 0 1)
    (:Default
      (CallFunction|StartTimeLine2 :!label _label))
    (:0
      (CallFunction|StartTimeLine1))
    (:1
      (goto _label))))

(event EventBeginPlay
  (CallFunction|ChooseTimeline))

(fn ConstructionScript)

(fn ScaleFlameIntensity
  (params (Intensity :type Float%20%28double-precision%29))
  (Rendering|Components|Light|SetIntensity (Variables|Default|GetFireLight) (* Intensity (Variables|Default|GetBaseIntensity))))